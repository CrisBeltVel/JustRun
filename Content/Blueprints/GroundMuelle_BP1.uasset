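; Endless-runner dock ground tile that populates itself with random obstacles and scenery on BeginPlay.
; SpawnObstacles uses chained random rolls to place props on three lanes, jittering the first lane's X, and lampposts, boats and water lilies at side positions.
; When the character overlaps BoxCollision, the game mode spawns the next tile and gains points.
; The player's walk speed then rises up to a cap, and the tile destroys itself after a delay.
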(event OnComponentBeginOverlap(BoxCollision)
  (params (OverlappedComponent :type Primitive%20Component%20Object%20Reference) (OtherActor :type Actor%20Object%20Reference) (OtherComp :type Primitive%20Component%20Object%20Reference) (OtherBodyIndex :type Integer) (bFromSweep :type Boolean) (SweepResult :type Hit%20Result%20Structure%20%28by%20ref%29))
  (Utilities|Casting|CastToThirdPersonCharacter OtherActor)
  (bind _asthird_person_game_mode (Utilities|Casting|CastToThirdPersonGameMode (Game|GetGameMode)))
  ;[1 1 1] Hace que la "BoxCollision" repita la plataforma indefinidamente
  (Default|SpawnGroundMuelles _asthird_person_game_mode)
  ;[1 1 1] Puntuación
  (bind _asthird_person_game_mode_2 (Utilities|Casting|CastToThirdPersonGameMode (Game|GetGameMode)))
  (bind _output_get (Variables|/Game/ThirdPersonBP/Blueprints/ThirdPersonGameMode.ThirdPersonGameMode_C|SetCurrentPoints _asthird_person_game_mode_2 (+ (Variables|/Game/ThirdPersonBP/Blueprints/ThirdPersonGameMode.ThirdPersonGameMode_C|GetCurrentPoints _asthird_person_game_mode_2) 100)))
  (Development|PrintString (Utilities|String|ToString(Integer) _output_get))
  ;[1 1 1] Cambio de velocidad
  (bind _asthird_person_character (Utilities|Casting|CastToThirdPersonCharacter (Game|GetPlayerCharacter 0)))
  ;;[1 1 1] Obtiener y  muestrar velocidad actual
  (bind _output_get_2 (Variables|/Script/Engine.CharacterMovementComponent|SetMaxWalkSpeed (Variables|/Script/Engine.Character|GetCharacterMovement _asthird_person_character) (Math|Float|Clamp(Float) (* (Variables|/Script/Engine.CharacterMovementComponent|GetMaxWalkSpeed (Variables|/Script/Engine.Character|GetCharacterMovement _asthird_person_character)) (Variables|Default|GetSpeedMultiplicationFactor)) 6e+02 (Variables|Default|GetMaxSpeed))))
  (Development|PrintString (Utilities|String|ToString(Float) _output_get_2))
  ;[1 1 1] Retardo previo a la destrucción de la plataforma
  (Utilities|FlowControl|Delay 2.0)
  ;[1 1 1] Destrucción de la plataforma
  (Actor|DestroyActor))

(event EventBeginPlay
  ;[1 1 1] Ejecuta los obstaculos
  (CallFunction|SpawnObstacles))

(event Collision|EventActorBeginOverlap
  (params (OtherActor :type Actor%20Object%20Reference)))

(event EventTick
  (params (DeltaSeconds :type Float%20%28single-precision%29)))

(fn ConstructionScript)

(fn SpawnObstacles
  (bind _returnvalue (Math|Random|RandomFloatinRange 0.0 1.0))
  (bind _returnvalue_2 (Math|Random|RandomFloatinRange 0.0 1.0))
  (bind _returnvalue_3 (Math|Random|RandomFloatinRange 0.0 1.0))
  (bind _returnvalue_4 (Math|Random|RandomFloatinRange 0.0 1.0))
  (bind _returnvalue_5 (Math|Random|RandomFloatinRange 0.0 1.0))
  (bind _returnvalue_6 (Math|Random|RandomFloatinRange 0.0 1.0))
  (bind _lane_lampara (Variables|Default|GetLane_Lampara))
  (bind _lane_lampara_2 (Variables|Default|GetLane_Lampara))
  (bind _lane2 (Variables|Default|GetLane2))
  (bind _lane0 (Variables|Default|GetLane0))
  (bind _lane1 (Variables|Default|GetLane1))
  (bind _lane_barco (Variables|Default|GetLane_BARCO))
  (bind _lane0_2 (Variables|Default|GetLane0))
  (bind _lane_loto (Variables|Default|GetLane_Loto))
  (bind _returnvalue_7 (Transformation|GetWorldTransform _lane_lampara))
  (bind _returnvalue_8 (Transformation|GetWorldTransform _lane_lampara_2))
  (bind _returnvalue_9 (Transformation|GetWorldTransform _lane1))
  (bind _returnvalue_10 (Transformation|GetWorldTransform _lane2))
  (bind _returnvalue_11 (Transformation|GetWorldTransform _lane_loto))
  (bind _returnvalue_12 (Transformation|GetWorldTransform _lane0_2))
  (bind _returnvalue_13 (Transformation|GetWorldTransform _lane_lampara))
  (bind _returnvalue_14 (Transformation|GetWorldTransform _lane0))
  (bind _returnvalue_15 (Transformation|GetWorldTransform _lane_barco))
  (bind _returnvalue_16 (Transformation|GetWorldTransform _lane_barco))
  (bind _returnvalue_17 (Transformation|GetWorldTransform _lane_loto))
  (Transformation|SetWorldLocation _lane0_2 (Math|Vector|MakeVector (+ (.x (.location _returnvalue_12)) (Math|Random|RandomFloatinRange 1.5e+02 5e+02)) (.y (.location _returnvalue_12)) (.z (.location _returnvalue_12))) false false)
  ;[1 1 1] Line0
  (if (Math|Float|InRange(Float) _returnvalue_5 0.0 0.1 false)
    _
    (elif (Math|Float|InRange(Float) _returnvalue_5 0.0 0.35)
      (Game|SpawnActorfromClass "/Game/Blueprints/ObstaculosMuelle/2Barriles_BP.2Barriles_BP_C" _returnvalue_14 "Undefined" 0 0)
      (elif (Math|Float|InRange(Float) _returnvalue_5 0.3 0.5)
        (Game|SpawnActorfromClass "/Game/Blueprints/ObstaculosMuelle/3Cajas_BP.3Cajas_BP_C" _returnvalue_14 "Undefined" 0 0)
        (elif (Math|Float|InRange(Float) _returnvalue_5 0.3 0.9)
          (Game|SpawnActorfromClass "/Game/Blueprints/ObstaculosMuelle/Silla2_BP.Silla2_BP_C" _returnvalue_14 "Undefined" 0 0)
          (elif (Math|Float|InRange(Float) _returnvalue_5 0.7 1.0)
            (Game|SpawnActorfromClass "/Game/Blueprints/Reconpensas/BP_Paleta.BP_Paleta_C" _returnvalue_14 "Undefined" 0 0))))))
  ;[1 1 1] Line1
  (if (Math|Float|InRange(Float) _returnvalue_3 0.0 0.1)
    ;[1 1 1] Line2
    (if (Math|Float|InRange(Float) _returnvalue_4 0.0 0.1) :!label _label
      _
      (elif (Math|Float|InRange(Float) _returnvalue_4 0.0 0.35)
        (Game|SpawnActorfromClass "/Game/Blueprints/ObstaculosMuelle/3Cajas_BP.3Cajas_BP_C" _returnvalue_10 "Undefined" 0 0)
        (elif (Math|Float|InRange(Float) _returnvalue_4 0.3 0.5)
          (Game|SpawnActorfromClass "/Game/Blueprints/ObstaculosMuelle/2Barriles_BP.2Barriles_BP_C" _returnvalue_10 "Undefined" 0 0)
          (elif (Math|Float|InRange(Float) _returnvalue_4 0.3 0.9)
            (Game|SpawnActorfromClass "/Game/Blueprints/ObstaculosMuelle/Silla_BP.Silla_BP_C" _returnvalue_10 "Undefined" 0 0)
            (elif (Math|Float|InRange(Float) _returnvalue_4 0.7 1.0)
              (Game|SpawnActorfromClass "/Game/Blueprints/Reconpensas/BP_Paleta.BP_Paleta_C" _returnvalue_10 "Undefined" 0 0))))))
    (if (Math|Float|InRange(Float) _returnvalue_2 0.0 0.0)
      _
      (elif (Math|Float|InRange(Float) _returnvalue_2 0.5 1.0)
        (Transformation|SetWorldLocation _lane_lampara (Math|Vector|MakeVector (.x (.location _returnvalue_13)) 247.0 (.z (.location _returnvalue_13))) false false)
        (Game|SpawnActorfromClass "/Game/Blueprints/ObstaculosMuelle/Farolas.Farolas_C" _returnvalue_7 "Undefined" 0 0)
        (elif true
          (Transformation|SetWorldLocation _lane_lampara_2 (Math|Vector|MakeVector (.x (.location _returnvalue_8)) -355.30307 (.z (.location _returnvalue_8))) false false)
          (Game|SpawnActorfromClass "/Game/Blueprints/ObstaculosMuelle/Farolas.Farolas_C" _returnvalue_7 "Undefined" 0 0))))
    (if (Math|Float|InRange(Float) _returnvalue_6 0.0 0.0)
      _
      (elif (Math|Float|InRange(Float) _returnvalue_6 0.5 1.0)
        (Transformation|SetWorldLocation _lane_barco (Math|Vector|MakeVector (.x (.location _returnvalue_16)) 573.0 (.z (.location _returnvalue_16))) false false)
        (Game|SpawnActorfromClass "/Game/Blueprints/ObstaculosMuelle/Barco_BP.Barco_BP_C" (Transformation|GetWorldTransform _lane_barco) "Undefined" 0 0 :!label _label_2)
        (elif (Math|Float|InRange(Float) _returnvalue_6 0.25 0.75)
          (Transformation|SetWorldLocation _lane_barco (Math|Vector|MakeVector (.x (.location _returnvalue_15)) -602.0 (.z (.location _returnvalue_15))) false false)
          (goto _label_2)
          (else
            _))))
    (if (not (Math|Float|InRange(Float) _returnvalue 0.0 0.0))
      (if (Math|Float|InRange(Float) _returnvalue 0.3 1.0)
        (Transformation|SetWorldLocation _lane_loto (Math|Vector|MakeVector (.x (.location _returnvalue_11)) 483.566284 (.z (.location _returnvalue_11))) false false)
        (Game|SpawnActorfromClass "/Game/AnimatedPondFish/Environment/Blueprints/BP_water_lily_01.BP_water_lily_01_C" (Transformation|GetWorldTransform _lane_loto) "Undefined" 0 0 :!label _label_3)
        (elif (Math|Float|InRange(Float) _returnvalue 0.25 0.75)
          (Transformation|SetWorldLocation _lane_loto (Math|Vector|MakeVector (.x (.location _returnvalue_17)) -862.042114 (.z (.location _returnvalue_17))) false false)
          (goto _label_3))))
    (elif (Math|Float|InRange(Float) _returnvalue_3 0.0 0.35)
      (Game|SpawnActorfromClass "/Game/Blueprints/ObstaculosMuelle/2Barriles_BP.2Barriles_BP_C" _returnvalue_9 "Undefined" 0 0)
      (goto _label)
      (elif (Math|Float|InRange(Float) _returnvalue_3 0.3 0.5)
        (Game|SpawnActorfromClass "/Game/Blueprints/ObstaculosMuelle/3Cajas_BP.3Cajas_BP_C" _returnvalue_9 "Undefined" 0 0)
        (elif (Math|Float|InRange(Float) _returnvalue_3 0.3 0.9)
          (Game|SpawnActorfromClass "/Game/Blueprints/Reconpensas/BP_Paleta.BP_Paleta_C" _returnvalue_9 "Undefined" 0 0)
          (goto _label)
          (elif (Math|Float|InRange(Float) _returnvalue_3 0.7 1.0)
            (Game|SpawnActorfromClass "/Game/Blueprints/Reconpensas/BP_Paleta.BP_Paleta_C" _returnvalue_9 "Undefined" 0 0)
            (goto _label)
            (else
              (goto _label))))))))