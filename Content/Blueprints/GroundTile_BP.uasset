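; Endless-runner ground tile that fills itself with random lane objects and recycles as the player advances.
; On BeginPlay, SpawnObstacles nudges Lane0 forward in X, then rolls fresh random chances per lane to spawn signs, carts, boards or shells; a Lane1 cart leaves Lane2 empty.
; Player overlap with BoxCollision has the GameMode spawn tiles and add points, raises walk speed within a clamp, then destroys the tile after a delay.
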(event OnComponentBeginOverlap(BoxCollision)
  (params (OverlappedComponent :type Primitive%20Component%20Object%20Reference) (OtherActor :type Actor%20Object%20Reference) (OtherComp :type Primitive%20Component%20Object%20Reference) (OtherBodyIndex :type Integer) (bFromSweep :type Boolean) (SweepResult :type Hit%20Result%20Structure%20%28by%20ref%29))
  (Utilities|Casting|CastToThirdPersonCharacter OtherActor)
  (bind _asthird_person_game_mode (Utilities|Casting|CastToThirdPersonGameMode (Game|GetGameMode)))
  ;[1 1 1] Hace que la "BoxCollision" repita la plataforma indefinidamente
  (Default|SpawnGroundTiles _asthird_person_game_mode)
  ;[1 1 1] Puntuación
  (bind _asthird_person_game_mode_2 (Utilities|Casting|CastToThirdPersonGameMode (Game|GetGameMode)))
  (bind _output_get (Variables|/Game/ThirdPersonBP/Blueprints/ThirdPersonGameMode.ThirdPersonGameMode_C|SetCurrentPoints _asthird_person_game_mode_2 (+ (Variables|/Game/ThirdPersonBP/Blueprints/ThirdPersonGameMode.ThirdPersonGameMode_C|GetCurrentPoints _asthird_person_game_mode_2) 100)))
  (Development|PrintString (Utilities|String|ToString(Integer) _output_get))
  ;[1 1 1] Cambio de velocidad
  (bind _asthird_person_character (Utilities|Casting|CastToThirdPersonCharacter (Game|GetPlayerCharacter 0)))
  ;;[1 1 1] Obtiener y  muestrar velocidad actual
  (bind _output_get_2 (Variables|/Script/Engine.CharacterMovementComponent|SetMaxWalkSpeed (Variables|/Script/Engine.Character|GetCharacterMovement _asthird_person_character) (Math|Float|Clamp(Float) (* (Variables|/Script/Engine.CharacterMovementComponent|GetMaxWalkSpeed (Variables|/Script/Engine.Character|GetCharacterMovement _asthird_person_character)) (Variables|Default|GetSpeedMultiplicationFactor)) 6e+02 (Variables|Default|GetMaxSpeed))))
  (Development|PrintString (Utilities|String|ToString(Float) _output_get_2))
  ;[1 1 1] Retardo previo a la destrucción de la plataforma
  (Utilities|FlowControl|Delay 2.0)
  ;[1 1 1] Destrucción de la plataforma
  (Actor|DestroyActor))

(event EventBeginPlay
  ;[1 1 1] Ejecuta los obstaculos
  (CallFunction|SpawnObstacles))

(event Collision|EventActorBeginOverlap
  (params (OtherActor :type Actor%20Object%20Reference)))

(event EventTick
  (params (DeltaSeconds :type Float%20%28single-precision%29)))

(fn ConstructionScript)

(fn SpawnObstacles
  (bind _returnvalue (Math|Random|RandomFloatinRange 0.0 1.0))
  (bind _returnvalue_2 (Math|Random|RandomFloatinRange 0.0 1.0))
  (bind _returnvalue_3 (Math|Random|RandomFloatinRange 0.0 1.0))
  (bind _lane0 (Variables|Default|GetLane0))
  (bind _lane0_2 (Variables|Default|GetLane0))
  (bind _lane1 (Variables|Default|GetLane1))
  (bind _lane2 (Variables|Default|GetLane2))
  (bind _returnvalue_4 (Transformation|GetWorldTransform _lane2))
  (bind _returnvalue_5 (Transformation|GetWorldTransform _lane1))
  (bind _returnvalue_6 (Transformation|GetWorldTransform _lane0))
  (bind _returnvalue_7 (Transformation|GetWorldTransform _lane0_2))
  (Transformation|SetWorldLocation _lane0 (Math|Vector|MakeVector (+ (.x (.location _returnvalue_6)) (Math|Random|RandomFloatinRange 1.5e+02 5e+02)) (.y (.location _returnvalue_6)) (.z (.location _returnvalue_6))) false false)
  ;[1 1 1] Line0
  (if (Math|Float|InRange(Float) _returnvalue_3 0.0 0.1 false)
    _
    (elif (Math|Float|InRange(Float) _returnvalue_3 0.0 0.35)
      (Game|SpawnActorfromClass "/Game/Blueprints/obstaculos/Letrero_BP.Letrero_BP_C" _returnvalue_7 "Undefined" 0 0)
      (elif (Math|Float|InRange(Float) _returnvalue_3 0.3 0.5)
        (Game|SpawnActorfromClass "/Game/Blueprints/obstaculos/Carrito_BP.Carrito_BP_C" _returnvalue_7 "Undefined" 0 0)
        (elif (Math|Float|InRange(Float) _returnvalue_3 0.3 0.9)
          (Game|SpawnActorfromClass "/Game/Blueprints/obstaculos/TablaSorft_BP.TablaSorft_BP_C" _returnvalue_7 "Undefined" 0 0)
          (elif (Math|Float|InRange(Float) _returnvalue_3 0.7 1.0)
            (Game|SpawnActorfromClass "/Game/Blueprints/Reconpensas/BP_Concha.BP_Concha_C" _returnvalue_7 "Undefined" 0 0))))))
  ;[1 1 1] Line1
  (if (Math|Float|InRange(Float) _returnvalue_2 0.0 0.1)
    ;[1 1 1] Line2
    (if (not (Math|Float|InRange(Float) _returnvalue 0.0 0.1)) :!label _label
      (if (Math|Float|InRange(Float) _returnvalue 0.0 0.35)
        (Game|SpawnActorfromClass "/Game/Blueprints/obstaculos/Letrero_BP.Letrero_BP_C" _returnvalue_4 "Undefined" 0 0)
        (elif (Math|Float|InRange(Float) _returnvalue 0.3 0.5)
          (Game|SpawnActorfromClass "/Game/Blueprints/obstaculos/Carrito_BP.Carrito_BP_C" _returnvalue_4 "Undefined" 0 0)
          (elif (Math|Float|InRange(Float) _returnvalue 0.3 0.9)
            (Game|SpawnActorfromClass "/Game/Blueprints/obstaculos/TablaSorft_BP.TablaSorft_BP_C" _returnvalue_4 "Undefined" 0 0)
            (elif (Math|Float|InRange(Float) _returnvalue 0.7 1.0)
              (Game|SpawnActorfromClass "/Game/Blueprints/Reconpensas/BP_Concha.BP_Concha_C" _returnvalue_4 "Undefined" 0 0))))))
    (elif (Math|Float|InRange(Float) _returnvalue_2 0.0 0.35)
      (Game|SpawnActorfromClass "/Game/Blueprints/obstaculos/Letrero_BP.Letrero_BP_C" _returnvalue_5 "Undefined" 0 0)
      (goto _label)
      (elif (Math|Float|InRange(Float) _returnvalue_2 0.3 0.5)
        (Game|SpawnActorfromClass "/Game/Blueprints/obstaculos/Carrito_BP.Carrito_BP_C" _returnvalue_5 "Undefined" 0 0)
        (elif (Math|Float|InRange(Float) _returnvalue_2 0.3 0.9)
          (Game|SpawnActorfromClass "/Game/Blueprints/Reconpensas/BP_Concha.BP_Concha_C" _returnvalue_5 "Undefined" 0 0)
          (goto _label)
          (elif (Math|Float|InRange(Float) _returnvalue_2 0.7 1.0)
            (Game|SpawnActorfromClass "/Game/Blueprints/Reconpensas/BP_Concha.BP_Concha_C" _returnvalue_5 "Undefined" 0 0)
            (goto _label)
            (else
              (goto _label))))))))